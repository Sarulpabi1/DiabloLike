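; BP_Dummy is an interactable, damageable dummy actor that displays the damage it receives.
; Any damage spawns a W_DamageAmount widget with the actor and damage amount and adds it to the viewport, with no health tracking.
; Clicking it sends itself to the player character as the interact target.
; Its Interactwith event does nothing, as the PrimaryAttack call is disconnected, and GetAttackRange returns zero.
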(event `self.ReceiveAnyDamage`
  (params (Damage :type "Float (single-precision)") (DamageType :type "DamageType Object Reference") (InstigatedBy :type "Controller Object Reference") (DamageCauser :type "Actor Object Reference"))
  (bind _returnvalue (`|CreateWidget` "/Game/UI/W_DamageAmount.W_DamageAmount_C" null self Damage))
  (`UserWidget.AddToViewport` _returnvalue 0))

(event `self.ReceiveActorOnClicked`
  (params (ButtonPressed :type "Key Structure"))
  (message `/Game/Systems/BP_InteractionInterface.SetInteractTarget` (`GameplayStatics.GetPlayerCharacter` 0) self))

(event `/Game/Systems/BP_InteractionInterface.InteractWith`
  (params (Character :type "Character Object Reference")))

(fn `GetAttackRange`
  (returns (Range :type "Float (double-precision)"))
  (return 0.0))

(fn `UserConstructionScript`)