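; BP_AbilityEffect_1 is a short-lived ability effect actor that deals a single burst of damage in front of itself.
; Shortly after BeginPlay it gathers actors overlapping its Sphere and uses a dot product against its forward vector to keep those in the front hemisphere.
; Those actors receive flat damage with the effect's owner as damage causer, and the effect destroys itself a few seconds later.
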(event `self.ReceiveBeginPlay`
  (`KismetSystemLibrary.Delay` 0.2)
  (for _array_element (`PrimitiveComponent.GetOverlappingActors` (`self.Sphere`) "/Script/Engine.Actor")
    (if (> (`KismetMathLibrary.Dot_VectorVector` (`KismetMathLibrary.GetDirectionUnitVector` (`self.K2_GetActorLocation`) (`self.K2_GetActorLocation` _array_element)) (`self.GetActorForwardVector`)) 0.0)
      (`GameplayStatics.ApplyDamage` _array_element 10.0 null (`self.GetOwner`))))
  (`KismetSystemLibrary.Delay` 3.0)
  (`self.K2_DestroyActor`))

(fn `UserConstructionScript`
  (`parent.UserConstructionScript`))