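; BP_AbilityParent is a base ability actor that activates on BeginPlay and sets its lifespan to its Cooldown value.
; Activation first checks that the owner's BP_StatsComponent reports enough of the cost stat, without deducting it here.
; If the check passes, it spawns each class in Effects at the Target's transform, falling back to the Caster's when no valid target exists.
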(event `self.ReceiveBeginPlay`
  (`self.ActivateAbility`)
  (`self.SetLifeSpan` (`self.Cooldown`)))

(event `ActivateAbility`
  (bind _target (`self.Target`))
  (if (`self.CanActivateAbility`)
    (for _array_element (`self.Effects`)
      (`|SpawnActorFromClass` _array_element (`KismetMathLibrary.SelectTransform` (`self.GetTransform` _target) (`self.GetTransform` (`self.Caster`)) (`KismetSystemLibrary.IsValid` _target)) "Undefined" "MultiplyWithRoot" null null))))

(fn `CanActivateAbility`
  (returns (ReturnValue :type Boolean))
  (bind _value (`/Game/Systems/BP_StatsComponent.QueryStat` (`self.GetComponentByClass` (`self.GetOwner`) "/Game/Systems/BP_StatsComponent.BP_StatsComponent_C") (`self.CostStat`)))
  (return (>= _value (`self.CostValue`))))

(fn `UserConstructionScript`)