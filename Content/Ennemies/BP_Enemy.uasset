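; Enemy character that chases the player on detection and gives up when it strays too far from where it spawned.
; A sphere overlap with the player raises walk speed, runs the chase behavior tree and writes the TargetActor blackboard key.
; While chasing, Tick compares distance to the spawn anchor against Range, then restores walk speed, switches to the wander tree and clears the target.
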(event `self.ReceiveBeginPlay`
  (`parent.ReceiveBeginPlay`)
  (set `self.Anchor` (`self.K2_GetActorLocation`))
  (set `CharacterMovementComponent.MaxWalkSpeed` (`self.Walk_Speed`) (`self.CharacterMovement`)))

(event `self.Sphere.OnComponentBeginOverlap`
  (params (OverlappedComponent :type "PrimitiveComponent Object Reference") (OtherActor :type "Actor Object Reference") (OtherComp :type "PrimitiveComponent Object Reference") (OtherBodyIndex :type Integer) (bFromSweep :type Boolean) (SweepResult :type "HitResult Structure (by ref)"))
  (if (== OtherActor (`GameplayStatics.GetPlayerCharacter` 0))
    (`self.StartChase`)
    (`BlackboardComponent.SetValueAsObject` (`AIBlueprintHelperLibrary.GetBlackboard` (`AIBlueprintHelperLibrary.GetAIController` self)) "TargetActor" OtherActor)))

(event `StartChase`
  (set `self.IsChasing` true)
  (set `CharacterMovementComponent.MaxWalkSpeed` (`self.Chase_Speed`) (`self.CharacterMovement`))
  (`AIController.RunBehaviorTree` (`AIBlueprintHelperLibrary.GetAIController` self) "/Game/Ennemies/AIBehavior/BT_Enemy_Chase.BT_Enemy_Chase"))

(event `StopChase`
  (set `self.IsChasing` false)
  (set `CharacterMovementComponent.MaxWalkSpeed` (`self.Walk_Speed`) (`self.CharacterMovement`))
  (`AIController.RunBehaviorTree` (`AIBlueprintHelperLibrary.GetAIController` self) "/Game/Ennemies/AIBehavior/BT_Enemy_Wander.BT_Enemy_Wander")
  (`BlackboardComponent.ClearValue` (`AIBlueprintHelperLibrary.GetBlackboard` (`AIBlueprintHelperLibrary.GetAIController` self)) "TargetActor"))

(event `self.ReceiveTick`
  (params (DeltaSeconds :type "Float (single-precision)"))
  (if (`self.IsChasing`)
    (if (> (`KismetMathLibrary.Vector_Distance` (`self.Anchor`) (`self.K2_GetActorLocation`)) (`self.Range`))
      (`self.StopChase`))))

(fn `UserConstructionScript`
  (`parent.UserConstructionScript`))