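; BP_StatsComponent is an actor component that holds an actor's stats and level, with helpers for combat damage math.
; Owner damage events subtract raw damage from Health through AlterBaseStats, which also reports whether the stat is depleted.
; QueryStat adds base and contribution map values, then applies a modifier; Strength feeds attack power for outgoing damage.
; A separate function scales damage by clamped level difference, but OnDamaged does not call it.
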(event `self.ReceiveBeginPlay`
  (add `Actor.OnTakeAnyDamage` (`self.GetOwner`) (delegate `OnDamaged`)))

(event `OnDamaged`
  (params (DamagedActor :type "Actor Object Reference") (Damage :type "Float (single-precision)") (DamageType :type "DamageType Object Reference") (InstigatedBy :type "Controller Object Reference") (DamageCauser :type "Actor Object Reference"))
  (`self.AlterBaseStats` "Health" (* Damage -1.0)))

(fn `AlterBaseStats`
  (params (Stat :type String) (Change :type "Float (double-precision)"))
  (returns (StatDepleted :type Boolean) (CurrentValue :type "Float (double-precision)"))
  (bind _basestats (`self.BaseStats`))
  (bind _stat (`local.Stat`))
  (bind (_value _returnvalue) (`BlueprintMapLibrary.Map_Find` (`self.BaseStats`) Stat))
  (bind _value_2 (`BlueprintMapLibrary.Map_Find` _basestats _stat))
  (if _returnvalue
    (`BlueprintMapLibrary.Map_Add` _basestats _stat (+ Change _value))
    (return (<= _value_2 0.0) _value_2)
    (else
      (`KismetSystemLibrary.PrintString` "Error : No valid stat available"))))

(fn `CalculateAttackPower`
  (returns (AttackPower :type "Float (double-precision)"))
  (bind _value (`self.QueryStat` "Strength"))
  (bind _output_get (set `self.AttackPower` _value))
  (return _output_get))

(fn `CalculateDamageDealt`
  (params (StartingDamage :type "Float (double-precision)") (Target :type "Actor Object Reference"))
  (returns (ReturnValue :type "Float (double-precision)"))
  (bind _attackpower (`self.CalculateAttackPower`))
  (return (* _attackpower (`KismetMathLibrary.NormalizeToRange` StartingDamage 0.0 20.0))))

(fn `CalculateDamageReduction`
  (params (StartingDamage :type "Float (double-precision)") (DamageCauser :type "Actor Object Reference") (DamageType :type "DamageType Object Reference"))
  (returns (ReturnValue :type "Float (double-precision)"))
  (locals (Local_LevelDifference :type Integer :default 0))
  (`|ExecutionSequence`
    (:`then_0`
      ;[1 1 1] Level Difference
      (bind _output_get (set `local.Local_LevelDifference` (`KismetMathLibrary.Clamp` (- (`/Game/Systems/BP_StatsComponent.Level` (`Actor.GetComponentByClass` DamageCauser "BP_StatsComponent_C")) (`self.Level`)) -6 6)))
      (return (* (`local.StartingDamage`) (+ 1.0 (/ (`KismetMathLibrary.Conv_IntToDouble` _output_get) 10.0)))))))

(fn `LevelUp`
  (set `self.Level` (`KismetMathLibrary.Clamp` (+ (`self.Level`) 1) 1 50)))

(fn `QueryStat`
  (params (Stat :type String))
  (returns (Value :type "Float (double-precision)"))
  (return (* (+ (`BlueprintMapLibrary.Map_Find` (`self.BaseStats`) Stat) (`BlueprintMapLibrary.Map_Find` (`self.StatContribution`) Stat)) (`BlueprintMapLibrary.Map_Find` (`self.StatModifiers`) Stat))))